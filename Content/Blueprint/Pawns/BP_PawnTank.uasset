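; Tank pawn Blueprint that puts a health bar on screen for the tank.
; BeginPlay creates a BP_HealthWidget and adds it to the viewport.
; GetHealthPercentage divides the Health component's current value by its maximum, and the result sets the widget's progress bar.
; The bar refreshes by polling every Tick, and OnDeath runs the same update without any other death handling.
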(event `self.ReceiveBeginPlay`
  (bind _returnvalue (`|CreateWidget` "/Game/Blueprint/Widgets/BP_HealthWidget.BP_HealthWidget_C"))
  (`UserWidget.AddToViewport` _returnvalue 0))

(event `self.OnDeath`
  (bind _returnvalue (`self.GetHealthPercentage` :!label _label))
  (bind _output_get (set `self.healthPercentage` _returnvalue))
  (`ProgressBar.SetPercent` (`/Game/Blueprint/Widgets/BP_HealthWidget.healthBarProgressBar` (stale `self.ReceiveBeginPlay` _returnvalue)) _output_get))

(event `self.ReceiveTick`
  (params (DeltaSeconds :type "Float (single-precision)"))
  (goto _label))

(fn `GetHealthPercentage`
  (returns (ReturnValue :type "Float (double-precision)"))
  (bind _health (`self.Health`))
  (return (/ (`HealthComponent.health` _health) (`HealthComponent.maxHealth` _health))))

(fn `UserConstructionScript`)